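; BP_Animal is a wildlife AI actor that wanders, flees from the player and gets drawn to lures.
; Roam chains AIMoveTo calls to random reachable points with random pauses, while flags track idle, fleeing and eating states.
; A trigger sphere starts Flee toward a random point away from the player.
; Other overlaps, when the player holds nothing, send it to "Lure"-tagged actors, which it eats and destroys before roaming again.
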(event `self.TriggerSphere.OnComponentBeginOverlap`
  (params (OverlappedComponent :type "PrimitiveComponent Object Reference") (OtherActor :type "Actor Object Reference") (OtherComp :type "PrimitiveComponent Object Reference") (OtherBodyIndex :type Integer) (bFromSweep :type Boolean) (SweepResult :type "HitResult Structure (by ref)"))
  ;[1 1 1] Collision with Player
  (if (== OtherActor (`self.Player`))
    (set `self.IsFleeing` true)
    (`MovementComponent.StopMovementImmediately` (`self.CharacterMovement`))
    (`self.Flee`)
    (else
      ;[1 1 1] Triggered by Lure
      (if (not (`/Game/ThirdPerson/Blueprints/BP_ThirdPersonCharacter.IsHolding` (`self.Player`)))
        (for _array_element (`self.GetOverlappingActors` "/Script/Engine.Actor")
          (bind _output_get (set `self.LureRef` _array_element))
          (if (`self.ActorHasTag` _output_get "Lure")
            (set `self.IsIdle` false)
            (`|AIMoveTo` self (`self.K2_GetActorLocation` _output_get) null 10.0
              (:`OnSuccess`
                (set `self.IsEatingLure` true)
                (`KismetSystemLibrary.Delay` 0.9)
                (`self.K2_DestroyActor` (`self.LureRef`))
                (set `self.IsEatingLure` false)
                (`KismetSystemLibrary.Delay` (`KismetMathLibrary.RandomFloatInRange` 2.0 10.0))
                (`self.Roam`)
                (break)))))))))

(event `self.ReceiveBeginPlay`
  ;[1 1 1] BeginPlay
  (bind _asbp_third_person_character (cast `/Game/ThirdPerson/Blueprints/BP_ThirdPersonCharacter` (`GameplayStatics.GetPlayerCharacter` 0)))
  (set `self.Player` _asbp_third_person_character)
  (`self.Roam`))

(event `self.TriggerSphere.OnComponentEndOverlap`
  (params (OverlappedComponent :type "PrimitiveComponent Object Reference") (OtherActor :type "Actor Object Reference") (OtherComp :type "PrimitiveComponent Object Reference") (OtherBodyIndex :type Integer))
  ;[1 1 1] Collision with Player
  (if (== OtherActor (`self.Player`))
    (set `self.IsFleeing` false)))

(event `Roam`
  ;[1 1 1] Roam AI
  (set `self.IsIdle` false)
  (`|AIMoveTo` self (`NavigationSystemV1.K2_GetRandomReachablePointInRadius` (`self.K2_GetActorLocation`) 1000.0 null null) null 120.0
    (:`OnSuccess`
      (set `self.IsIdle` true)
      (`KismetSystemLibrary.Delay` (`KismetMathLibrary.RandomFloatInRange` 2.0 10.0))
      (`self.Roam`))))

(event `Flee`
  (bind _returnvalue (`self.K2_GetActorLocation`))
  ;[1 1 1] Flee AI
  (set `self.IsIdle` false)
  (`|AIMoveTo` self (`NavigationSystemV1.K2_GetRandomReachablePointInRadius` (`KismetMathLibrary.MakeVector` (.x (+ _returnvalue (* (`KismetMathLibrary.GetForwardVector` (`KismetMathLibrary.FindLookAtRotation` _returnvalue (`self.K2_GetActorLocation` (`self.Player`)))) -800.0))) (.y (+ _returnvalue (* (`KismetMathLibrary.GetForwardVector` (`KismetMathLibrary.FindLookAtRotation` _returnvalue (`self.K2_GetActorLocation` (`self.Player`)))) -800.0))) (.z _returnvalue)) 500.0 null null) null 120.0
    (:`OnSuccess`
      (set `self.IsFleeing` false)
      (`KismetSystemLibrary.Delay` (`KismetMathLibrary.RandomFloatInRange` 2.0 10.0))
      (`self.Roam`))))

(fn `UserConstructionScript`)