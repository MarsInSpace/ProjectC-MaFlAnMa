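; BP_Creature_ChangeMesh is a creature actor that changes shape when the player character overlaps its Sphere.
; On begin overlap with BP_ThirdPersonCharacter, the Creature mesh becomes Shape_NarrowCapsule and loses collision.
; Any end overlap restores the placeholder mesh after a ten-second Delay, without checking the actor.
; The node re-enabling collision is unconnected, so collision stays off once triggered.
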(event `self.Sphere.OnComponentBeginOverlap`
  (params (OverlappedComponent :type "PrimitiveComponent Object Reference") (OtherActor :type "Actor Object Reference") (OtherComp :type "PrimitiveComponent Object Reference") (OtherBodyIndex :type Integer) (bFromSweep :type Boolean) (SweepResult :type "HitResult Structure (by ref)"))
  ;[1 1 1] Change Color on Collision
  (cast `/Game/ThirdPerson/Blueprints/BP_ThirdPersonCharacter` OtherActor)
  (`StaticMeshComponent.SetStaticMesh` (`self.Creature`) "/Game/StarterContent/Shapes/Shape_NarrowCapsule.Shape_NarrowCapsule")
  (`PrimitiveComponent.SetCollisionEnabled` (`self.Creature`) "NoCollision"))

(event `self.Sphere.OnComponentEndOverlap`
  (params (OverlappedComponent :type "PrimitiveComponent Object Reference") (OtherActor :type "Actor Object Reference") (OtherComp :type "PrimitiveComponent Object Reference") (OtherBodyIndex :type Integer))
  ;[1 1 1] Changing Back Color Going Out of Collision
  (`KismetSystemLibrary.Delay` 10.0)
  (`StaticMeshComponent.SetStaticMesh` (`self.Creature`) "/Game/Angy/StaticMesh_Creature_Placeholder.StaticMesh_Creature_Placeholder"))

(fn `UserConstructionScript`)