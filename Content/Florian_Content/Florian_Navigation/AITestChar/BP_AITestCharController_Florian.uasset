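; AI controller for a test character that runs BT_AITestChar_Florian on BeginPlay and reacts to perception updates about the player.
; HandleSightSense filters stimuli by comparing their sense class to AISenseConfig_Sight (the config class, not AISense_Sight) and ignores actors other than player 0.
; It sets Blackboard TargetActor while the player is sensed.
; On loss, it clears TargetActor and stores the stimulus location as LastKnownPosition.
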(event `self.AIPerception.OnTargetPerceptionUpdated`
  (params (Actor :type "Actor Object Reference") (Stimulus :type "AIStimulus Structure"))
  (`self.HandleSightSense` Actor Stimulus))

(event `self.ReceiveBeginPlay`
  (`self.RunBehaviorTree` "/Game/Florian_Content/Florian_Navigation/AITestChar/BT_AITestChar_Florian.BT_AITestChar_Florian"))

(fn `HandleSightSense`
  (params (Actor :type "Actor Object Reference") (Stimulus :type "AIStimulus Structure"))
  (bind (_stimulus_age _stimulus_expirationage _stimulus_strength _stimulus_stimuluslocation _stimulus_receiverlocation _stimulus_tag _stimulus_bsuccessfullysensed) (break `AIStimulus` (`local.Stimulus`)))
  (bind _returnvalue (`AIPerceptionSystem.GetSenseClassForStimulus` Stimulus))
  (if (== _returnvalue "/Script/AIModule.AISenseConfig_Sight")
    (if (== (`local.Actor`) (`GameplayStatics.GetPlayerCharacter` 0))
      (`BlackboardComponent.SetValueAsObject` (`self.Blackboard`) "TargetActor" (`KismetMathLibrary.SelectObject` (`GameplayStatics.GetPlayerCharacter` 0) null _stimulus_bsuccessfullysensed))
      (if (not _stimulus_bsuccessfullysensed)
        (`BlackboardComponent.SetValueAsVector` (`self.Blackboard`) "LastKnownPosition" _stimulus_stimuluslocation))
      (else
        (return)))
    (else
      (return))))

(fn `UserConstructionScript`)