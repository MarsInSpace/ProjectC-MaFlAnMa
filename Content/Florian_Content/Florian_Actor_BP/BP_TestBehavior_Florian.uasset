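; Test behavior actor that makes a creature flee and vanish when the third-person character enters its trigger box, then reappear later.
; Begin overlap slides the Creature component away over two seconds, then hides it and disables collision.
; End overlap by any actor waits six seconds, slides it to the opposite offset, then restores visibility and collision.
; Disconnected material-swap nodes, including a dust particle material, never run.
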(event `self.Box.OnComponentBeginOverlap`
  (params (OverlappedComponent :type "PrimitiveComponent Object Reference") (OtherActor :type "Actor Object Reference") (OtherComp :type "PrimitiveComponent Object Reference") (OtherBodyIndex :type Integer) (bFromSweep :type Boolean) (SweepResult :type "HitResult Structure (by ref)"))
  ;[1 1 1] Disappear + ReAppear Creature
  (cast `/Game/ThirdPerson/Blueprints/BP_ThirdPersonCharacter` OtherActor)
  (`KismetSystemLibrary.MoveComponentTo` (`self.Creature`) (1000.0 0.0 0.0) (struct) false false 2.0)
  (`SceneComponent.SetVisibility` (`self.Creature`) false false)
  (`PrimitiveComponent.SetCollisionEnabled` (`self.Creature`) "NoCollision"))

(event `self.Box.OnComponentEndOverlap`
  (params (OverlappedComponent :type "PrimitiveComponent Object Reference") (OtherActor :type "Actor Object Reference") (OtherComp :type "PrimitiveComponent Object Reference") (OtherBodyIndex :type Integer))
  ;[1 1 1] Disappear + ReAppear Creature
  (`KismetSystemLibrary.Delay` 6.0)
  (`KismetSystemLibrary.MoveComponentTo` (`self.Creature`) (-1000.0 0.0 0.0) (struct) true false 2.0)
  (`SceneComponent.SetVisibility` (`self.Creature`) true false)
  (`PrimitiveComponent.SetCollisionEnabled` (`self.Creature`) "QueryAndPhysics"))

(fn `UserConstructionScript`)