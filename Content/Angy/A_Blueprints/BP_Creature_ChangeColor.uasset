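; Creature actor that changes color and becomes passable when the third-person player character comes near it.
; When the player character enters its Sphere, the Creature component switches to the changing material and disables its collision.
; Any end overlap on the Sphere, with no player check, waits a fixed delay, then restores the original material and query-and-physics collision.
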(event `self.Sphere.OnComponentBeginOverlap`
  (params (OverlappedComponent :type "PrimitiveComponent Object Reference") (OtherActor :type "Actor Object Reference") (OtherComp :type "PrimitiveComponent Object Reference") (OtherBodyIndex :type Integer) (bFromSweep :type Boolean) (SweepResult :type "HitResult Structure (by ref)"))
  ;[1 1 1] Change Color on Collision
  (cast `/Game/ThirdPerson/Blueprints/BP_ThirdPersonCharacter` OtherActor)
  (`PrimitiveComponent.SetMaterial` (`self.Creature`) 0 "/Game/Angy/Materials/M_Creature_Changing.M_Creature_Changing")
  (`PrimitiveComponent.SetCollisionEnabled` (`self.Creature`) "NoCollision"))

(event `self.Sphere.OnComponentEndOverlap`
  (params (OverlappedComponent :type "PrimitiveComponent Object Reference") (OtherActor :type "Actor Object Reference") (OtherComp :type "PrimitiveComponent Object Reference") (OtherBodyIndex :type Integer))
  ;[1 1 1] Changing Back Color Going Out of Collision
  (`KismetSystemLibrary.Delay` 4.0)
  (`PrimitiveComponent.SetMaterial` (`self.Creature`) 0 "/Game/Angy/Materials/M_Creature.M_Creature")
  (`PrimitiveComponent.SetCollisionEnabled` (`self.Creature`) "QueryAndPhysics"))

(fn `UserConstructionScript`)