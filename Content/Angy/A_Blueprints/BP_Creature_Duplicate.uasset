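; BP_Creature_Duplicate is a creature actor that duplicates itself when the third-person character overlaps its Sphere component.
; Each overlap spawns another copy at a fixed X offset, turns off that copy's Sphere collision and prints a debug message.
; BeginPlay re-enables Sphere collision after a short delay, so new copies can duplicate in turn.
; The end-overlap handler is empty, and mesh-swap and mesh-collision nodes are left unconnected.
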(event `self.ReceiveBeginPlay`
  (`KismetSystemLibrary.Delay` 5.0)
  (`PrimitiveComponent.SetCollisionEnabled` (`self.Sphere`) "QueryAndPhysics"))

(event `self.Sphere.OnComponentBeginOverlap`
  (params (OverlappedComponent :type "PrimitiveComponent Object Reference") (OtherActor :type "Actor Object Reference") (OtherComp :type "PrimitiveComponent Object Reference") (OtherBodyIndex :type Integer) (bFromSweep :type Boolean) (SweepResult :type "HitResult Structure (by ref)"))
  (bind (_returnvalue_location _returnvalue_rotation _returnvalue_scale) (`KismetMathLibrary.BreakTransform` (`self.GetTransform`)))
  ;[1 1 1] Duplicating On Collision
  (cast `/Game/ThirdPerson/Blueprints/BP_ThirdPersonCharacter` OtherActor)
  (bind _returnvalue (`|SpawnActorFromClass` "BP_Creature_Duplicate_C" (`KismetMathLibrary.MakeTransform` (+ _returnvalue_location (100.0 0.0 0.0)) _returnvalue_rotation _returnvalue_scale) "Undefined" "OverrideRootScale" null null))
  (`PrimitiveComponent.SetCollisionEnabled` (`/Game/Angy/A_Blueprints/BP_Creature_Duplicate.Sphere` _returnvalue) "NoCollision")
  (`KismetSystemLibrary.PrintText` "Hello"))

(event `self.Sphere.OnComponentEndOverlap`
  (params (OverlappedComponent :type "PrimitiveComponent Object Reference") (OtherActor :type "Actor Object Reference") (OtherComp :type "PrimitiveComponent Object Reference") (OtherBodyIndex :type Integer))
  ;[1 1 1] Changing Back Color Going Out of Collision
)

(fn `UserConstructionScript`)