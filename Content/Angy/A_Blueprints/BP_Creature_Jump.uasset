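; BP_Creature_Jump is a creature that hops when the third-person player character enters its trigger sphere.
; Two chained MoveComponentTo calls ease the Creature component up and back to its relative origin, then its collision is switched off.
; Any end overlap on the sphere, with no character check, restores query and physics collision after a delay of several seconds.
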(event `self.Sphere.OnComponentBeginOverlap`
  (params (OverlappedComponent :type "PrimitiveComponent Object Reference") (OtherActor :type "Actor Object Reference") (OtherComp :type "PrimitiveComponent Object Reference") (OtherBodyIndex :type Integer) (bFromSweep :type Boolean) (SweepResult :type "HitResult Structure (by ref)"))
  ;[1 1 1] Jump on Collision
  (cast `/Game/ThirdPerson/Blueprints/BP_ThirdPersonCharacter` OtherActor)
  (`KismetSystemLibrary.MoveComponentTo` (`self.Creature`) (0.0 0.0 200.0) (struct) true false 0.3)
  (`KismetSystemLibrary.MoveComponentTo` (`self.Creature`) (0.0 0.0 0.0) (struct) false true 0.5)
  (`PrimitiveComponent.SetCollisionEnabled` (`self.Creature`) "NoCollision"))

(event `self.Sphere.OnComponentEndOverlap`
  (params (OverlappedComponent :type "PrimitiveComponent Object Reference") (OtherActor :type "Actor Object Reference") (OtherComp :type "PrimitiveComponent Object Reference") (OtherBodyIndex :type Integer))
  ;[1 1 1] Turn on Collision Again
  (`KismetSystemLibrary.Delay` 7.0)
  (`PrimitiveComponent.SetCollisionEnabled` (`self.Creature`) "QueryAndPhysics"))

(fn `UserConstructionScript`)