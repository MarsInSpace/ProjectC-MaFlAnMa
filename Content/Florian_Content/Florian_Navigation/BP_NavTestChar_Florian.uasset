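; Test NPC character that wanders the navigation mesh on its own, starting at BeginPlay.
; A self-repeating MoveNPC event picks a random reachable point around the current location and runs AI Move To, pausing after success or retrying almost immediately on failure.
; Two helper functions, not called in this graph, toggle the mouse cursor and input mode, with focus on a Gallery widget.
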(event `self.ReceiveBeginPlay`
  (`self.MoveNPC`))

(event `MoveNPC`
  ;[1 1 1] NPC Movement
  (bind _output_get (set `self.Random Location` (`NavigationSystemV1.K2_GetRandomReachablePointInRadius` (`self.K2_GetActorLocation`) 1000.0 null null)))
  (`|AIMoveTo` self _output_get null
    (:`OnSuccess`
      (`KismetSystemLibrary.Delay` 4.0)
      (`self.MoveNPC`))
    (:`OnFail`
      (`KismetSystemLibrary.Delay` 0.1)
      (`self.MoveNPC`))))

(fn `DisableMouseCursor`
  (bind _returnvalue (`GameplayStatics.GetPlayerController` 0))
  (`WidgetBlueprintLibrary.SetInputMode_GameOnly` _returnvalue)
  (set `PlayerController.bShowMouseCursor` false _returnvalue))

(fn `EnableMouseCursor`
  (bind _returnvalue (`GameplayStatics.GetPlayerController` 0))
  (`WidgetBlueprintLibrary.SetInputMode_GameAndUIEx` _returnvalue (`self.Gallery`))
  (set `PlayerController.bShowMouseCursor` true _returnvalue))

(fn `UserConstructionScript`)